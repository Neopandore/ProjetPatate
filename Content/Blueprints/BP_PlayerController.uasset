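; BP_PlayerController is the player controller for a Mastermind game, managing the game and start-screen widgets.
; On BeginPlay it adds UMG_Mastermind to the viewport with UMG_StartGame layered above it.
; The IStopGame event shows the start screen again, while IStartGame forwards a start message to the game widget.
; The AddUMG helper reuses a valid widget reference or creates one before adding it to the viewport.
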(event EventBeginPlay
  (bind _umgref_out (CallFunction|AddUMG "/Game/Blueprints/Mastermind/Widgets/UMG_Mastermind.UMG_Mastermind_C" 0 (Variables|Default|GetGameUMG)))
  (Variables|Default|SetGameUMG _umgref_out)
  (bind _umgref_out_2 (CallFunction|AddUMG "/Game/Blueprints/Mastermind/Widgets/UMG_StartGame.UMG_StartGame_C" 1 (Variables|Default|GetStartUMG)))
  (Variables|Default|SetStartUMG _umgref_out_2))

(event EventIStartGame
  (Class|BPiUMGInterface|IStartGame(Message) (Variables|Default|GetGameUMG)))

(event EventIStopGame
  (bind _umgref_out (CallFunction|AddUMG "/Game/Blueprints/Mastermind/Widgets/UMG_StartGame.UMG_StartGame_C" 1 (Variables|Default|GetStartUMG)))
  (Variables|Default|SetStartUMG _umgref_out))

(fn ConstructionScript)

(fn AddUMG
  (params (UMG :type User%20Widget%20Class%20Reference) (ZOrder :type Integer) (UMGRef :type User%20Widget%20Object%20Reference))
  (bind _output_get (LocalVariables|SetUMGRef_Local UMGRef))
  (Utilities|IsValid _output_get
    (:Is%20Valid
      _)
    (:Is%20Not%20Valid
      (bind _returnvalue (UserInterface|CreateWidget UMG))
      (LocalVariables|SetUMGRef_Local _returnvalue)))
  (UserInterface|Viewport|AddtoViewport (LocalVariables|GetUMGRef_Local) ZOrder)
  (return (LocalVariables|GetUMGRef_Local)))